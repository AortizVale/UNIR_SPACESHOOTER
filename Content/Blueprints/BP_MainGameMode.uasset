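; BP_MainGameMode is the game mode for a space game, tracking progress, kills, level and turret unlocks.
; It caches the player character and HUD at start, increments progress every tick and forwards player death to the HUD.
; Each enemy kill counts toward a level increase on every second kill.
; While the player lacks a turret, kills also fill the HUD turret meter, activating the turret at the required count.
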(event `self.ReceiveBeginPlay`
  (bind _asbp_space_s_character (cast `/Game/Player/BP_SpaceS_Character` (`GameplayStatics.GetPlayerCharacter` 0))
    (:`then`
      (set `self.m_spaceCharacterController` _asbp_space_s_character))
    (:`CastFailed`
      _))
  (bind _asbp_space_s_hud (cast `/Game/UI/BP_SpaceS_HUD` (`PlayerController.GetHUD` (`GameplayStatics.GetPlayerController` 0))))
  (set `self.m_spaceS_HUD` _asbp_space_s_hud))

(event `self.ReceiveTick`
  (params (DeltaSeconds :type "Float (single-precision)"))
  (set `self.Progress` (+ (`self.Progress`) (`self.IncrementPerTick`))))

(event `PlayerDead`
  (bind _asbp_space_s_hud (cast `/Game/UI/BP_SpaceS_HUD` (`PlayerController.GetHUD` (`GameplayStatics.GetPlayerController` 0))))
  (`/Game/UI/BP_SpaceS_HUD.PlayerKilled` _asbp_space_s_hud))

(event `EnemyDestroyed`
  (`self.TurretFunction`)
  (bind _output_get (set `self.EnemiesDestroyed` (+ (`self.EnemiesDestroyed`) 1)))
  (if (== (mod _output_get 2) 0)
    (set `self.Level` (+ (`self.Level`) 1))))

(fn `TurretFunction`
  (bind _enemiesrequiredforturret (`self.EnemiesRequiredForTurret`))
  (if (not (`/Game/Player/BP_SpaceS_Character.HasTurret` (`self.m_spaceCharacterController`)))
    (bind _output_get (set `self.EnemiesKilledForTurret` (+ (`self.EnemiesKilledForTurret`) 1)))
    (`/Game/UI/BP_SpaceS_HUD.SetTurretProgress` (`self.m_spaceS_HUD`) (/ (`KismetMathLibrary.Conv_IntToDouble` _output_get) (`KismetMathLibrary.Conv_IntToDouble` _enemiesrequiredforturret)))
    (if (>= _output_get _enemiesrequiredforturret)
      (set `self.EnemiesKilledForTurret` 0)
      (`KismetSystemLibrary.PrintString` "Turret Activated")
      (`/Game/Player/BP_SpaceS_Character.ActivateTurret` (`self.m_spaceCharacterController`)))))

(fn `UserConstructionScript`)