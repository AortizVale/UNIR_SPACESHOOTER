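; BP_EnemyBaseHSin is an enemy Blueprint variant that gives its movement a horizontal wave pattern.
; Each Tick runs the parent logic, accumulates Time, then overwrites MovementVector's X with a cosine scaled by Frequency, Amplitude and DeltaSeconds, keeping Y and Z.
; The cosine acts as a per-frame step, so summed steps would trace a sine path.
; BeginPlay, overlap and construction logic only call the parent.
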(event `self.ReceiveBeginPlay`
  (`parent.ReceiveBeginPlay`))

(event `self.ReceiveActorBeginOverlap`
  (params (OtherActor :type "Actor Object Reference"))
  (`parent.ReceiveActorBeginOverlap` OtherActor))

(event `self.ReceiveTick`
  (params (DeltaSeconds :type "Float (single-precision)"))
  (bind (_movementvector_x _movementvector_y _movementvector_z) (`KismetMathLibrary.BreakVector` (`self.MovementVector`)))
  (`parent.ReceiveTick` DeltaSeconds)
  (bind _output_get (set `self.Time` (+ (`self.Time`) DeltaSeconds)))
  (set `self.MovementVector` (`KismetMathLibrary.MakeVector` (* (* (`KismetMathLibrary.Cos` (* _output_get (`self.Frequency`))) (`self.Amplitude`)) DeltaSeconds) _movementvector_y _movementvector_z)))

(fn `UserConstructionScript`
  (`parent.UserConstructionScript`))